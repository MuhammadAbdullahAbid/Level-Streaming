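; BP_LevelStreamVolume is a trigger volume that swaps streamed levels behind a loading screen.
; A box overlap binds load events, shows a WBP_Loading widget and, after a short delay, calls LoadLevel with a level name and location.
; Progress events feed the widget's percentage, and completion unloads the named previous level and removes the widget.
; The overlap neither filters actors nor checks its load-started flag.
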(event `self.Box.OnComponentBeginOverlap`
  (params (OverlappedComponent :type "PrimitiveComponent Object Reference") (OtherActor :type "Actor Object Reference") (OtherComp :type "PrimitiveComponent Object Reference") (OtherBodyIndex :type Integer) (bFromSweep :type Boolean) (SweepResult :type "HitResult Structure (by ref)"))
  (add `self.OnLevelLoading` (delegate `On Level Loading`))
  (add `self.OnLoadComplete` (delegate `On Load Complete`))
  (set `self.bIsLoadStarted` true)
  (bind _returnvalue (`|CreateWidget` "/Game/WBP_Loading.WBP_Loading_C"))
  (bind _output_get (set `self.WBP_Loading` _returnvalue))
  (`UserWidget.AddToViewport` _output_get 0)
  (`KismetSystemLibrary.Delay` 2.0)
  (`self.LoadLevel` (`self.LoadLevelName`) (`self.Location`))
  (bind _returnvalue_2 (`self.IsLevelLoaded` (`self.LoadLevelName`)))
  (set `self.bIsLevelLoaded` _returnvalue_2))

(event `On Level Loading` :!signature `self.OnLevelLoading`
  (params (Percentage :type "Float (single-precision) (by ref)"))
  (bind _output_get (set `/Game/WBP_Loading.LoadPercentage` Percentage (`self.WBP_Loading`)))
  (if (>= _output_get 100.0)
    (clear `self.OnLevelLoading`)))

(event `On Load Complete`
  (`self.UnLoadLevel` (`self.UnLoadLevelName`))
  (`Widget.RemoveFromParent` (`self.WBP_Loading`))
  (clear `self.OnLoadComplete`))

(fn `UserConstructionScript`)